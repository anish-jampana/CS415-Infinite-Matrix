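; BP_Enemy is an enemy obstacle that damages the player on collision and awards score when shot.
; Hitting BP_Player reduces its clamped Health, plays a world camera shake and destroys the Enemy component, triggering the restart display and zeroing ForwardSpeed at zero health.
; An overlapping BP_Projectile adds to its shooter's Score and destroys the component.
; RandomizeEnemy, not called within this Blueprint, randomly offsets and rotates the component.
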(event `self.Enemy.OnComponentHit`
  (params (HitComponent :type "PrimitiveComponent Object Reference") (OtherActor :type "Actor Object Reference") (OtherComp :type "PrimitiveComponent Object Reference") (NormalImpulse :type "Vector Structure") (Hit :type "HitResult Structure (by ref)"))
  (bind _asbp_player (cast `/Game/InfiniteMatrix/Blueprints/BP_Player` OtherActor))
  (set `/Game/InfiniteMatrix/Blueprints/BP_Player.Health` (`KismetMathLibrary.FClamp` (- (`/Game/InfiniteMatrix/Blueprints/BP_Player.Health` _asbp_player) 10.0) 0.0 100.0) _asbp_player)
  (`GameplayStatics.PlayWorldCameraShake` "/Game/InfiniteMatrix/Blueprints/BP_Shake.BP_Shake_C" (`self.K2_GetActorLocation` _asbp_player) 0.0 500.0)
  (`ActorComponent.K2_DestroyComponent` (`self.Enemy`))
  (if (== (`/Game/InfiniteMatrix/Blueprints/BP_Player.Health` _asbp_player) 0.0)
    (`/Game/InfiniteMatrix/Blueprints/BP_Player.DisplayRestart` _asbp_player)
    (set `/Game/InfiniteMatrix/Blueprints/BP_Player.ForwardSpeed` 0.0 _asbp_player)))

(event `self.Enemy.OnComponentBeginOverlap`
  (params (OverlappedComponent :type "PrimitiveComponent Object Reference") (OtherActor :type "Actor Object Reference") (OtherComp :type "PrimitiveComponent Object Reference") (OtherBodyIndex :type Integer) (bFromSweep :type Boolean) (SweepResult :type "HitResult Structure (by ref)"))
  (bind _asbp_projectile (cast `/Game/InfiniteMatrix/Blueprints/BP_Projectile` OtherActor))
  (bind _player_shoot (`/Game/InfiniteMatrix/Blueprints/BP_Projectile.Player Shoot` _asbp_projectile))
  (set `/Game/InfiniteMatrix/Blueprints/BP_Player.Score` (+ (`/Game/InfiniteMatrix/Blueprints/BP_Player.Score` _player_shoot) 5.0) _player_shoot)
  (`ActorComponent.K2_DestroyComponent` (`self.Enemy`)))

(fn `Randomize Enemy`
  (`SceneComponent.K2_AddLocalOffset` (`self.Enemy`) (`KismetMathLibrary.MakeVector` (`KismetMathLibrary.RandomFloatInRange` 800.0 2000.0) (`KismetMathLibrary.RandomFloatInRange` -300.0 300.0) (`KismetMathLibrary.RandomFloatInRange` -300.0 300.0)) false false)
  (`SceneComponent.K2_AddLocalRotation` (`self.Enemy`) (struct :`Yaw` 180.0) false false))

(fn `UserConstructionScript`)